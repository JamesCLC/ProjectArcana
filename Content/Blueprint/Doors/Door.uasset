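; Sliding door actor that opens when any actor overlaps it and closes when an overlap ends, unless locked.
; A timeline slides the Door component along relative X, with sounds when movement starts and finishes.
; UnlockDoor clears Locked, swaps the indicator material, recolors two point lights cyan and sets collision to query-only, also running at construction for unlocked doors.
; Separate helper functions toggle or set those lights' visibility.
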(event Collision|EventActorBeginOverlap
  (params (OtherActor :type Actor%20Object%20Reference))
  (if (not (Variables|Default|GetLocked))
    (Audio|PlaySoundatLocation "/Game/Sounds/Environment/OpenDoor.OpenDoor" (Transformation|GetActorLocation))
    (bind _newtrack_0 (Timeline|Timeline_0 Play)
      (:Update
        (Transformation|SetRelativeLocation (Variables|Default|GetDoor) (Math|Vector|MakeVector _newtrack_0 0.0 0.0) false false))
      (:Finished
        (Audio|PlaySoundatLocation "/Game/Sounds/Environment/DoorStop.DoorStop" (Transformation|GetActorLocation))))))

(event Collision|EventActorEndOverlap
  (params (OtherActor :type Actor%20Object%20Reference))
  (if (not (Variables|Default|GetLocked))
    (Audio|PlaySoundatLocation "/Game/Sounds/Environment/OpenDoor.OpenDoor" (Transformation|GetActorLocation))
    (bind _newtrack_0 (Timeline|Timeline_0 Reverse)
      (:Update
        (Transformation|SetRelativeLocation (Variables|Default|GetDoor) (Math|Vector|MakeVector _newtrack_0 0.0 0.0) false false))
      (:Finished
        (Audio|PlaySoundatLocation "/Game/Sounds/Environment/DoorStop.DoorStop" (Transformation|GetActorLocation))))))

(event EventTick
  (params (DeltaSeconds :type Float%20%28single-precision%29)))

(fn ConstructionScript
  (if (not (Variables|Default|GetLocked))
    (CallFunction|UnlockDoor)))

(fn UnlockDoor
  (Rendering|Material|SetMaterial (Variables|Default|GetDoorLight) 0 "/Game/Blueprint/Doors/DoorUnlocked.DoorUnlocked")
  (Collision|SetCollisionEnabled (Variables|Default|GetDoor) "QueryOnly")
  (for _array_element (Utilities|Array|MakeArray (Variables|Default|GetPointLight1) (Variables|Default|GetPointLight))
    (Rendering|Components|Light|SetLightColor _array_element "(R=0.000000,G=0.763963,B=1.000000,A=1.000000)" true))
  (Variables|Default|SetLocked false))

(fn NewFunction0
  (bind _isa (Utilities|FlowControl|FlipFlop)
    (:A
      _)
    (:B
      _))
  (Rendering|SetVisibility (Variables|Default|GetPointLight) (not _isa) false)
  (Rendering|SetVisibility (Variables|Default|GetPointLight1) (not _isa) false))

(fn ToggleDoorLights
  (bind _isa (Utilities|FlowControl|FlipFlop)
    (:A
      _)
    (:B
      _))
  (Rendering|SetVisibility (Variables|Default|GetPointLight) (not _isa) false)
  (Rendering|SetVisibility (Variables|Default|GetPointLight1) (not _isa) false))
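; UIPath is an actor that draws a given path as a chain of spline meshes along a spline.
; The construction script pre-allocates spline points and mesh segments based on PointCount.
; GeneratePath reuses that pool, moving points to the path's local-space positions, collapsing excess points onto the path end and refitting each mesh segment.
; GeneratePath_0 is an empty stub holding disconnected rebuild logic.
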(event EventBeginPlay)

(event Collision|EventActorBeginOverlap
  (params (OtherActor :type Actor%20Object%20Reference)))

(event EventTick
  (params (DeltaSeconds :type Float%20%28single-precision%29)))

(fn ConstructionScript
  (bind _spline (Variables|Default|GetSpline))
  (bind _pointcount (Variables|Default|GetPointCount))
  (for _index (range 0 _pointcount)
    (Spline|AddSplinePoint (Variables|Default|GetSpline) (Math|Vector|MakeVector 0.0 0.0 0.0) "Local" true))
  (for _index_2 (range 0 (+ _pointcount 2))
    (bind _returnvalue (AddComponent|AddSplineMeshComponent false))
    (Utilities|Array|Add (Variables|Default|GetSplineMeshArray) _returnvalue)
    (SplineMesh|SetStartandEnd _returnvalue (.Location (Spline|GetLocationandTangentatSplinePoint _spline _index_2 "Local")) (.Tangent (Spline|GetLocationandTangentatSplinePoint _spline _index_2 "Local")) (.Location (Spline|GetLocationandTangentatSplinePoint _spline (+ _index_2 1) "Local")) (.Tangent (Spline|GetLocationandTangentatSplinePoint _spline (+ _index_2 1) "Local")) true :!class /Script/Engine.SplineMeshComponent)))

(fn GeneratePath
  (params (Path :type Array%20of%20Vectors))
  (bind _spline (Variables|Default|GetSpline))
  (bind _spline_2 (Variables|Default|GetSpline))
  (for _index (range 0 (- (Spline|GetNumberOfSplinePoints (Variables|Default|GetSpline)) 1))
    (if (> (Utilities|Array|Length Path) _index) ; If we've reached the end of the path, set all the excess points at the path end.
      (Spline|SetLocationatSplinePoint (Variables|Default|GetSpline) _index (Utilities|Array|Get(acopy) Path _index) "Local" true)
      (else
        (Spline|SetLocationatSplinePoint _spline _index (.Location (Spline|GetLocationandTangentatSplinePoint _spline (- _index 1) "Local")) "Local" true)))
    (SplineMesh|SetStartandEnd (Utilities|Array|Get(acopy) (Variables|Default|GetSplineMeshArray) _index) (.Location (Spline|GetLocationandTangentatSplinePoint _spline_2 _index "Local")) (.Tangent (Spline|GetLocationandTangentatSplinePoint _spline_2 _index "Local")) (.Location (Spline|GetLocationandTangentatSplinePoint _spline_2 (+ _index 1) "Local")) (.Tangent (Spline|GetLocationandTangentatSplinePoint _spline_2 (+ _index 1) "Local")) true :!class /Script/Engine.SplineMeshComponent)))

(fn GeneratePath0
  (params (Path :type Array%20of%20Vectors)))
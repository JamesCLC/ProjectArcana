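; DoorCables is a spline-based cable actor whose colour can be switched to signal an unlock.
; The construction script adds a spline mesh component for each segment between spline points, fits it to the local positions and tangents, and stores it in MeshArray.
; Unlock gives every stored mesh a dynamic material instance with its Colour parameter set to light blue; the event graph is empty.
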(event EventBeginPlay)

(event Collision|EventActorBeginOverlap
  (params (OtherActor :type Actor%20Object%20Reference)))

(event EventTick
  (params (DeltaSeconds :type Float%20%28single-precision%29)))

(fn ConstructionScript
  (bind _spline (Variables|Default|GetSpline))
  (for _index (range 0 (- (Spline|GetNumberOfSplinePoints (Variables|Default|GetSpline)) 2))
    (bind _returnvalue (AddComponent|AddSplineMeshComponent false))
    (Utilities|Array|Add (Variables|Default|GetMeshArray) _returnvalue) ; Stores the mesh for later.
    (SplineMesh|SetStartandEnd _returnvalue (.Location (Spline|GetLocationandTangentatSplinePoint _spline _index "Local")) (.Tangent (Spline|GetLocationandTangentatSplinePoint _spline _index "Local")) (.Location (Spline|GetLocationandTangentatSplinePoint _spline (+ _index 1) "Local")) (.Tangent (Spline|GetLocationandTangentatSplinePoint _spline (+ _index 1) "Local")) true :!class /Script/Engine.SplineMeshComponent)))

(fn Unlock
  (for _array_element (Variables|Default|GetMeshArray)
    (bind _returnvalue (Rendering|Material|CreateDynamicMaterialInstance (Rendering|Material|GetMaterial _array_element 0) :!class /Script/Engine.KismetMaterialLibrary))
    (Rendering|Material|SetVectorParameterValue _returnvalue "Colour" "(R=0.000000,G=0.658457,B=1.000000,A=1.000000)" :!class /Script/Engine.MaterialInstanceDynamic)
    (Rendering|Material|SetMaterial _array_element 0 _returnvalue)))